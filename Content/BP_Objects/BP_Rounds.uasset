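; Round manager actor that tracks score and round progress over a set of targets.
; CheckWinRound updates the score, then counts the round as won when no target in Targets is still active.
; A win prints the results, resets the score, advances the round and plays a ping, lighting a point light until a timeline finishes.
; Once the third round is won, it destroys all the targets.
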(event Custom|CheckWinRound
  (params (Score :type Integer))
  (Variables|Default|SetScore (+ Score (Variables|Default|GetScore)))
  (Variables|Default|SetCanWin true)
  (bind _array_element (Utilities|Array|ForEachLoopwithBreak (Variables|Default|GetTargets) :!label _label)
    (:LoopBody
      (if (Variables|/Game/BP_Objects/BP_Target.BP_Target_C|GetIsActive _array_element)
        (Variables|Default|SetCanWin false)
        (goto _label Break)))
    (:Completed
      (if (Variables|Default|GetCanWin)
        ;[0.15 0.15 0.15 0.5] Win round
        (Development|PrintString (Utilities|String|ToString(Integer) (Variables|Default|GetScore)) true true "(R=0.000000,G=0.660000,B=1.000000,A=1.000000)" 5.0)
        (Development|PrintString "Score:" true true "(R=0.000000,G=0.660000,B=1.000000,A=1.000000)" 5.0)
        (Development|PrintString (Utilities|String|ToString(Integer) (Variables|Default|GetRound)) true true "(R=0.000000,G=0.660000,B=1.000000,A=1.000000)" 5.0)
        (Development|PrintString "You Won Round:" true true "(R=0.000000,G=0.660000,B=1.000000,A=1.000000)" 5.0)
        (Variables|Default|SetScore 0)
        (Rendering|Components|Light|SetIntensity (Variables|Default|GetPointLight) 5e+03)
        (bind _output_get (Variables|Default|SetRound (+ (Variables|Default|GetRound) 1)))
        (bind _array_element_2 (Utilities|Array|ForEachLoopwithBreak (Variables|Default|GetTargets))
          (:LoopBody
            (if (> _output_get 3)
              (Actor|DestroyActor _array_element_2)))
          (:Completed
            (Audio|PlaySoundatLocation "/Engine/EngineSounds/1kSineTonePing.1kSineTonePing" (Transformation|GetActorLocation) "0, 0, 0" 1.0 1.0 0.0 0 0 0 0)
            (Timeline|Timeline PlayFromStart
              (:Finished
                (Rendering|Components|Light|SetIntensity (Variables|Default|GetPointLight) 0.0)))))))))

(event EventBeginPlay
  (Variables|Default|SetRound 1)
  (Variables|Default|SetScore 0)
  (Rendering|Components|Light|SetIntensity (Variables|Default|GetPointLight) 0.0))

(fn ConstructionScript)