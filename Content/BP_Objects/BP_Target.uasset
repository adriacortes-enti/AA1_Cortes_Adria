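; Shooting-range style target actor that picks a random color on BeginPlay, which sets its material, hit points and score value.
; Each Hit while active spawns an explosion and removes HP; at zero it reports its value to BP_Rounds via CheckWinRound.
; It then plays chained timelines to rotate away, wait out a cooldown and rotate back, reactivating with the same color and restored HP.
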(event Custom|HideTarget
  ;[0.15 0.15 0.15 0.5] Get hit
  (Audio|PlaySoundatLocation "/Game/StarterContent/Audio/Collapse_Cue.Collapse_Cue" (Transformation|GetActorLocation) "0, 0, 0" 1.0 1.0 0.0 0 0 0 0)
  (Variables|Default|SetIsActive false)
  (Default|CheckWinRound (Variables|Default|GetRoundBP) (Variables|Default|GetValue))
  (bind _newtrack_1 (Timeline|HideAnim PlayFromStart)
    (:Update
      (Transformation|SetActorRelativeRotation (Math|Rotator|MakeRotator 0.0 0.0 _newtrack_1)))
    (:Finished
      (Timeline|Cooldown PlayFromStart
        (:Finished
          (bind _newtrack_1_2 (Timeline|ShowAnim ReverseFromEnd)
            (:Update
              (Transformation|SetActorRelativeRotation (Math|Rotator|MakeRotator 0.0 0.0 _newtrack_1_2)))
            (:Finished
              (CallFunction|ColorEvent))))))))

(event Custom|ColorEvent
  (bind _staticmesh (Variables|Default|GetStaticMesh))
  ;[0.15 0.15 0.15 0.5] Update values depending on the color
  (switch Utilities|FlowControl|Switch|SwitchonE_Colors (Variables|Default|GetColor)
    (:NewEnumerator1
      (Rendering|Material|SetMaterial _staticmesh 2 "/Game/Models/M_red.M_red")
      (Variables|Default|SetHP 1)
      (Variables|Default|SetValue 1))
    (:NewEnumerator2
      (Rendering|Material|SetMaterial _staticmesh 2 "/Game/Models/M_Yellow.M_Yellow")
      (Variables|Default|SetHP 2)
      (Variables|Default|SetValue 2))
    (:NewEnumerator0
      (Rendering|Material|SetMaterial _staticmesh 2 "/Game/Models/M_Blue.M_Blue")
      (Variables|Default|SetHP 3)
      (Variables|Default|SetValue 3)))
  (Variables|Default|SetIsActive true))

(event EventBeginPlay
  ;[0.15 0.15 0.15 0.5] Assign color
  (Variables|Default|SetColor (Utilities|Enum|ByteToEnumE_Colors (Math|Conversions|ToByte(Integer) (Math|Random|RandomInteger (|GetNumEnumEntries)))))
  (CallFunction|ColorEvent)
  (bind _returnvalue (Actor|GetActorOfClass "/Game/BP_Objects/BP_Rounds.BP_Rounds_C"))
  (Variables|Default|SetRoundBP _returnvalue))

(event Collision|EventHit
  (params (MyComp :type Primitive%20Component%20Object%20Reference) (Other :type Actor%20Object%20Reference) (OtherComp :type Primitive%20Component%20Object%20Reference) (bSelfMoved :type Boolean) (HitLocation :type Vector :default "0, 0, 0") (HitNormal :type Vector :default "0, 0, 0") (NormalImpulse :type Vector :default "0, 0, 0") (Hit :type Hit%20Result%20Structure%20%28by%20ref%29))
  (if (Variables|Default|GetIsActive)
    (bind _output_get (Variables|Default|SetHP (- (Variables|Default|GetHP) 1)))
    (Effects|SpawnEmitteratLocation "/Game/StarterContent/Particles/P_Explosion.P_Explosion" (Transformation|GetActorLocation))
    (if (<= _output_get 0)
      (CallFunction|HideTarget))))

(fn ConstructionScript)